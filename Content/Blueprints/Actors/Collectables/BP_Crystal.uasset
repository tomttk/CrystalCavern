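; BP_Crystal is a collectable crystal that is drawn to the player on touch and then disappears.
; When the player pawn overlaps it, the crystal stores its location and plays a timeline that lerps it toward the pawn's current location using a smoothed alpha.
; The target is re-read each update so the crystal follows a moving player, and the actor destroys itself when the timeline finishes.
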(event Collision|EventActorBeginOverlap
  (params (OtherActor :type Actor%20Object%20Reference))
  (bind _returnvalue (Game|Player|GetPlayerPawn 0))
  (if (== OtherActor _returnvalue)
    (Variables|Default|SetLerp%20Start%20Location (Transformation|GetActorLocation))
    (bind _smooth_lerp_alpha (Timeline|Alpha%20Blend%20Timeline Play)
      (:Update
        (Transformation|SetActorLocation (Math|Vector|Lerp(Vector) (Variables|Default|GetLerp%20Start%20Location) (Transformation|GetActorLocation _returnvalue) _smooth_lerp_alpha) false false))
      (:Finished
        (Actor|DestroyActor)))))

(fn ConstructionScript)