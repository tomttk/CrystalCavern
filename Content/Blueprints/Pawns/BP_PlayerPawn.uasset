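; Player pawn that rolls a physics mesh by applying torque from the forward/backward and right/left input axes, scaled by an acceleration multiplier.
; The camera fades in on BeginPlay.
; Any damage triggers a one-shot restart that fades out screen and audio, waits briefly, then reopens the current level.
; A helper function sets the spring arm's length and world pitch to adjust the camera.
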(event EventBeginPlay
  ;[1 1 1] Camera Fade In
  (CameraFades|StartCameraFade :self (Game|GetPlayerCameraManager 0) :FromAlpha 1.0 :Duration 3.0))

(event Game|Damage|EventAnyDamage
  (params (Damage :type Float%20%28single-precision%29) (DamageType :type Damage%20Type%20Object%20Reference) (InstigatedBy :type Controller%20Object%20Reference) (DamageCauser :type Actor%20Object%20Reference))
  (Utilities|RestartLevel))

(event Input|AxisEvents|InputAxisMoveForwards/Backwards
  (params (AxisValue :type Float%20%28single-precision%29))
  ;[1 1 1] Movement
  (Class|PrimitiveComponent|AddTorqueinRadians (Variables|Default|GetMesh) (Math|Vector|MakeVector 0.0 (* AxisValue (Variables|Default|GetAcceleration%20Multiplier)) 0.0) "None" true))

(event Input|AxisEvents|InputAxisMoveRight/Left
  (params (AxisValue :type Float%20%28single-precision%29))
  ;[1 1 1] Movement
  (Class|PrimitiveComponent|AddTorqueinRadians (Variables|Default|GetMesh) (Math|Vector|MakeVector (* AxisValue (Variables|Default|GetAcceleration%20Multiplier)) 0.0 0.0) "None" true))

(fn ConstructionScript)

(fn AdjustSpringArm
  (params (Distance :type Float%20%28double-precision%29) (Pitch :type Float%20%28double-precision%29))
  (bind _springarm (Variables|Default|GetSpringArm))
  (Variables|/Script/Engine.SpringArmComponent|SetTargetArmLength _springarm Distance)
  (Transformation|SetWorldRotation _springarm (Math|Rotator|MakeRotator 0.0 Pitch 0.0) false false))